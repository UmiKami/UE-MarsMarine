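; BP_HealthPickup is a pickup that heals a BP_Marine that overlaps it, unless that player's health is already full.
; On a successful overlap it adds HealthToAdd and sets ShouldKillActor, which makes Tick run KillActor.
; KillActor drives the item particle's ParticleScale parameter from a float curve over time and destroys the actor once the curve evaluates to zero.
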(event `self.ReceiveTick`
  (params (DeltaSeconds :type "Float (single-precision)"))
  (if (`self.ShouldKillActor`)
    (`self.KillActor` DeltaSeconds)))

(event `self.OnActorOverlap`
  (params (OverlappedComponent :type "PrimitiveComponent Object Reference") (OtherActor :type "Actor Object Reference") (OtherComp :type "PrimitiveComponent Object Reference") (OtherBodyIndex :type Integer) (bFromSweep :type Boolean) (SweepResult :type "HitResult Structure (by ref)"))
  (bind _asbp_marine (cast `/Game/Blueprints/Pawns/BP_Marine` OtherActor))
  (if (not (`MM_CharacterBase.IsPlayerHealthFull` _asbp_marine))
    (`MM_CharacterBase.AddHealth` _asbp_marine (`self.HealthToAdd`))
    (set `self.ShouldKillActor` true)))

(fn `KillActor`
  (params (DeltaTime :type "Float (double-precision)"))
  (bind _returnvalue (`KismetMathLibrary.GetRuntimeFloatCurveValue` (`self.Curve`) (`self.CurrentParticleScaleInTime`)))
  (`FXSystemComponent.SetFloatParameter` (`self.ItemParticle`) "ParticleScale" _returnvalue)
  (set `self.CurrentParticleScaleInTime` (+ DeltaTime (`self.CurrentParticleScaleInTime`)))
  (if (== _returnvalue 0.0)
    (`self.K2_DestroyActor`)))

(fn `UserConstructionScript`)