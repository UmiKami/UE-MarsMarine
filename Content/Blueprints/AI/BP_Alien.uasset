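; BP_Alien is an enemy alien with a head health bar and forward melee attack against BP_Marine.
; Hurt events update the cached widget, while death hides it, dissolves the mesh's dynamic material on Tick and destroys the actor after a delay.
; Attacks use a sphere trace ignoring fellow aliens to damage the player.
; Helpers check attack range and spawn another alien at a random TargetPoint, though nothing here calls them.
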(event `self.ReceiveBeginPlay`
  (add `self.AlienIsDeadSignature` (delegate `AlienIsDeadSignature_Event`)))

(event `AlienIsDeadSignature_Event` :!signature `self.AlienIsDeadSignature`
  (params (IsDead :type Boolean) (AlienInstance :type "MM_AlienBase Object Reference"))
  (`self.HideHealthBarWhenDead`)
  (`KismetSystemLibrary.Delay` 5.0)
  (`self.K2_DestroyActor`))

(event `self.ReceiveTick`
  (params (DeltaSeconds :type "Float (single-precision)"))
  (if (`self.IsDead`)
    (`self.DissolveAlien` DeltaSeconds)))

(event `self.AlienHasBeenHurt`
  (`/Engine/EditorBlueprintResources/StandardMacros.IsValid` (`self.WBPHealthBar`)
    (:`Is Valid`
      _)
    (:`Is Not Valid`
      (bind _aswbp_head_heealth_bar (cast `/Game/UI/Overhead/WBP_HeadHeealthBar` (`WidgetComponent.GetWidget` (`self.AlienHealthBarWidget`))))
      (set `self.WBPHealthBar` _aswbp_head_heealth_bar)))
  (set `/Game/UI/Overhead/WBP_HeadHeealthBar.AlienHealth` (/ (`self.Health`) (`self.MaxHealth`)) (`self.WBPHealthBar`)))

(fn `DissolveAlien`
  (params (DeltaTime :type "Float (double-precision)"))
  (bind _returnvalue (`MaterialInstanceDynamic.K2_GetScalarParameterValue` (`self.SpiderMaterial`) "Dissolve"))
  (`MaterialInstanceDynamic.SetScalarParameterValue` (`self.SpiderMaterial`) "Dissolve" (`KismetMathLibrary.FInterpTo` _returnvalue 1.0 DeltaTime 1.0)))

(fn `GetRandomSpawnPoint`
  (returns (SpawnPoint :type "TargetPoint Object Reference"))
  (bind _outactors (`GameplayStatics.GetAllActorsOfClass` "/Script/Engine.TargetPoint"))
  (return (`KismetArrayLibrary.Array_Random` _outactors)))

(fn `HideHealthBarWhenDead`
  (`Widget.SetVisibility` (`WidgetComponent.GetWidget` (`self.AlienHealthBarWidget`)) "Hidden"))

(fn `IsWithinAttackRange`
  (returns (IsWithinAttackRange :type Boolean))
  (return (<= (`self.GetDistanceTo` (`GameplayStatics.GetPlayerCharacter` 0)) (`self.AttackRange`))))

(fn `SpawnAlien`
  (bind _spawnpoint (`self.GetRandomSpawnPoint`))
  (`/Engine/EditorBlueprintResources/StandardMacros.IsValid` _spawnpoint
    (:`Is Valid`
      (`|SpawnActorFromClass` (`GameplayStatics.GetObjectClass` self) (`self.GetTransform` _spawnpoint) "Undefined" "MultiplyWithRoot" null null))))

(fn `TryHitPlayer`
  (bind _returnvalue (`self.K2_GetActorLocation`))
  (if (not (`self.IsDead`))
    (bind _outactors (`GameplayStatics.GetAllActorsOfClass` "BP_Alien_C"))
    (set `self.Actors to Ignore` _outactors)
    (bind _outhits (`KismetSystemLibrary.SphereTraceMulti` _returnvalue (+ _returnvalue (* (`self.GetActorForwardVector`) (`self.AttackRange`))) (`self.DamageBoxRadius`) "TraceTypeQuery1" false (`self.Actors to Ignore`)))
    (for _array_element _outhits
      (cast `/Game/Blueprints/Pawns/BP_Marine` (`.HitActor` (`GameplayStatics.BreakHitResult` _array_element)))
      (`self.DamagePlayer`)
      (break))))

(fn `UserConstructionScript`
  (bind _returnvalue (`PrimitiveComponent.CreateDynamicMaterialInstance` (`self.Mesh`) 0 null "None"))
  (set `self.SpiderMaterial` _returnvalue))