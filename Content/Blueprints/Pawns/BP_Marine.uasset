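; BP_Marine is the marine pawn Blueprint, which tracks enemy kills by listening for alien deaths.
; On BeginPlay it binds to the death dispatcher of every existing BP_Alien.
; It also subscribes to BP_MarsGameMode's spawn dispatcher to bind each alien spawned at runtime.
; Both death handlers call IncrementEnemyKillCount, which is not defined in this graph.
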(event `self.ReceiveBeginPlay`
  (bind _outactors (`GameplayStatics.GetAllActorsOfClass` "/Game/Blueprints/AI/BP_Alien.BP_Alien_C"))
  (for _array_element _outactors
    (add `MM_AlienBase.AlienIsDeadSignature` _array_element (delegate `AlienIsDeadSignature_Event`)))
  ;[0.15 0 0.03099 0.5] Ensures we subscribe to the death event of every spider that is spawned at runtime
  (bind _asbp_mars_game_mode (cast `/Game/Blueprints/Game/BP_MarsGameMode` (`GameplayStatics.GetGameMode`)))
  (add `/Game/Blueprints/Game/BP_MarsGameMode.AlienHasBeenSpawned` _asbp_mars_game_mode (delegate `AlienHasBeenSpawned_Event`)))

(event `AlienIsDeadSignature_Event`
  (params (IsDead :type Boolean) (AlienInstance :type "MM_AlienBase Object Reference"))
  (`self.IncrementEnemyKillCount`))

(event `AlienHasBeenSpawned_Event`
  (params (Alien :type "/Game/Blueprints/AI/BP_Alien Object Reference"))
  ;[0.15 0 0.03099 0.5] Ensures we subscribe to the death event of every spider that is spawned at runtime
  (add `MM_AlienBase.AlienIsDeadSignature` Alien (delegate `AlienIsDeadSignature_Event_0`)))

(event `self.ReceiveTick`
  (params (DeltaSeconds :type "Float (single-precision)")))

(event `AlienIsDeadSignature_Event_0`
  (params (IsDead :type Boolean) (AlienInstance :type "MM_AlienBase Object Reference"))
  ;[0.15 0 0.03099 0.5] Ensures we subscribe to the death event of every spider that is spawned at runtime
  (`self.IncrementEnemyKillCount`))

(fn `UserConstructionScript`)