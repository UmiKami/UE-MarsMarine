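; BP_MissionAreaVolume is a volume that marks the mission area and kills the player marine for staying outside it too long.
; Overlap begin and end toggle OutsideMissionArea on any overlapping BP_Marine.
; Leaving starts a timer of SecondsBeforePlayerDeath and re-entering clears it.
; When it expires, KillPlayer deals MaxHealth damage to player character 0, whichever marine triggered the timer.
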(event `self.ReceiveActorBeginOverlap`
  (params (OtherActor :type "Actor Object Reference"))
  (bind _asbp_marine (cast `/Game/Blueprints/Pawns/BP_Marine` OtherActor))
  (set `MM_CharacterBase.bOutsideMissionArea` false _asbp_marine)
  (`KismetSystemLibrary.K2_ClearTimer` null "KillPlayer"))

(event `self.ReceiveActorEndOverlap`
  (params (OtherActor :type "Actor Object Reference"))
  (bind _asbp_marine (cast `/Game/Blueprints/Pawns/BP_Marine` OtherActor))
  (set `MM_CharacterBase.bOutsideMissionArea` true _asbp_marine)
  (`KismetSystemLibrary.K2_SetTimer` null "KillPlayer" (`self.SecondsBeforePlayerDeath`)))

(fn `KillPlayer`
  (bind _asbp_marine (cast `/Game/Blueprints/Pawns/BP_Marine` (`GameplayStatics.GetPlayerCharacter` 0)))
  (`GameplayStatics.ApplyDamage` _asbp_marine (`MM_CharacterBase.MaxHealth` _asbp_marine) null self))

(fn `UserConstructionScript`)