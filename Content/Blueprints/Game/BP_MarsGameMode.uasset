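; Game mode for the Mars game that spawns aliens in waves and tracks the ones still alive.
; The SpawnWaveSignature delegate triggers SpawnAlien, which places a BP_Alien at a random TargetPoint, binds its death delegate, broadcasts the spawn and decrements the remaining spawn count.
; When AlienHasDied runs, it removes that alien from RemainingAliens and calls TrySpawningNextWave, whose logic lives outside this graph.
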(event `self.ReceiveBeginPlay`
  (add `self.SpawnWaveSignature` (delegate `SpawnWaveSignature_Event`)))

(event `SpawnWaveSignature_Event`
  (`self.SpawnAlien`))

(event `AlienHasDied`
  (params (IsDead :type Boolean) (AlienInstance :type "MM_AlienBase Object Reference"))
  (`KismetArrayLibrary.Array_RemoveItem` (`self.RemainingAliens`) AlienInstance)
  (`self.TrySpawningNextWave`))

(fn `GetRandomSpawnPoint`
  (returns (SpawnPoint :type "TargetPoint Object Reference"))
  (bind _outactors (`GameplayStatics.GetAllActorsOfClass` "/Script/Engine.TargetPoint"))
  (return (`KismetArrayLibrary.Array_Random` _outactors)))

(fn `SpawnAlien`
  (bind _spawnpoint (`self.GetRandomSpawnPoint`))
  (`/Engine/EditorBlueprintResources/StandardMacros.IsValid` _spawnpoint
    (:`Is Valid`
      (bind _returnvalue (`|SpawnActorFromClass` "/Game/Blueprints/AI/BP_Alien.BP_Alien_C" (`self.GetTransform` _spawnpoint) "Undefined" "MultiplyWithRoot" null null))
      (`/Engine/EditorBlueprintResources/StandardMacros.IsValid` _returnvalue
        (:`Is Valid`
          (`KismetArrayLibrary.Array_Add` (`self.RemainingAliens`) _returnvalue)
          (add `MM_AlienBase.AlienIsDeadSignature` _returnvalue (`|CreateDelegate` :!event `AlienHasDied`))
          (`self.AlienHasBeenSpawned` _returnvalue)
          (`/Engine/EditorBlueprintResources/StandardMacros.DecrementInt` (`self.AlienSpawnsRemaining`)))))))

(fn `UserConstructionScript`)